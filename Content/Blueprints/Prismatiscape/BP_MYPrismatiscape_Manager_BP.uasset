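; Manager actor for the Prismatiscape Niagara grid simulation of deform, surface, wind and water effects in an area following the player pawn's root component.
; On BeginPlay it sizes render targets, sets grid parameters and applies style profiles.
; Each post-tick it evaluates timed deform and wind capsule pulses, then feeds them and interaction bubbles to Niagara arrays.
; Grid origins snap to texel increments, with pixel offsets sent to Niagara and locations to a Material Parameter Collection.
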(event Custom|ApplyPrismatiscapeStyleProfile
  (params (Profile :type Prismatiscape%20Style%20Profile%20Object%20Reference))
  (Default|ApplyProfile Profile (Variables|Default|GetNiagara))
  (CallFunction|ReplaceCurrentStyleProfile Profile))

(event Custom|ReInitNiagaraSystem)

(event Custom|ReapplyAllStyleProfiles
  (for _array_element (Variables|Default|GetCurrentSimulationStyles)
    (Default|ApplyProfile _array_element (Variables|Default|GetNiagara))))

(event Custom|OnRefershj
  (CallFunction|ReapplyAllStyleProfiles))

(event EventBeginPlay
  (Utilities|FlowControl|Sequence
    (:then_0
      (CallFunction|SetInitialParams)
      (CallFunction|ReapplyAllStyleProfiles)
      (CallFunction|InitComponenttoFollow))
    (:then_1
      (Utilities|FlowControl|Delay 0.5)
      (Actor|Tick|SetActorTickEnabled true))))

(event EventPostTick
  (CallFunction|ProcessAllPulses)
  (CallFunction|CalculateRTPositionsandOffsets)
  (CallFunction|SetGridTickVariables))

(fn ConstructionScript)

(fn RemoveComponentfromDrawList
  (params (Component :type Old%20BP%20Prismatiscape%20Deform%20Component%20Object%20Reference))
  (Utilities|Array|RemoveItem (Variables|DataArrays|GetDeformComponentArray) Component))

(fn AddComponenttoWindList
  (params (Component :type Old%20BP%20Prismatiscape%20Deform%20Component%20Object%20Reference%20%28by%20ref%29))
  (Utilities|Array|AddUnique (Variables|DataArrays|GetDeformComponentArray) Component))

(fn ProcessPulses
  (params (ThisPulseArray :type Array%20of%20Prismatiscape%20Pulse%20Struct%20Structures) (StartLocAndRad :type Array%20of%20Vector%204%20Structures) (EndLocAndRad :type Array%20of%20Vector%204%20Structures) (StartVelAndStr :type Array%20of%20Vector%204%20Structures) (EndVelAndStr :type Array%20of%20Vector%204%20Structures))
  (for _index (range 0 (Utilities|Array|LastIndex ThisPulseArray))
    (if (== (.Duration (Utilities|Struct|BreakPrismatiscape_PulseStruct (Utilities|Array|Get(acopy) ThisPulseArray _index))) 0.0)
      (Utilities|Array|Add (LocalVariables|GetIntsToDelete) _index)
      (Utilities|FlowControl|Sequence
        (:then_0
          (Utilities|Array|Add StartLocAndRad (.CapsuleStartLocationAndRadius (Utilities|Struct|BreakPrismatiscape_Draw_Shape (.DrawShape (Utilities|Struct|BreakPrismatiscape_PulseStruct (Utilities|Array|Get(acopy) ThisPulseArray _index)))))))
        (:then_1
          (Utilities|Array|Add EndLocAndRad (.CapsuleEndLocationAndRadius (Utilities|Struct|BreakPrismatiscape_Draw_Shape (.DrawShape (Utilities|Struct|BreakPrismatiscape_PulseStruct (Utilities|Array|Get(acopy) ThisPulseArray _index)))))))
        (:then_2
          (Utilities|Array|Add StartVelAndStr (.CapsuleStartVelocityAndStrength (Utilities|Struct|BreakPrismatiscape_Draw_Shape (.DrawShape (Utilities|Struct|BreakPrismatiscape_PulseStruct (Utilities|Array|Get(acopy) ThisPulseArray _index)))))))
        (:then_3
          (Utilities|Array|Add EndVelAndStr (.CapsuleEndVelocityAndStrength (Utilities|Struct|BreakPrismatiscape_Draw_Shape (.DrawShape (Utilities|Struct|BreakPrismatiscape_PulseStruct (Utilities|Array|Get(acopy) ThisPulseArray _index))))))))
      (else
        (if (< (/ (- (Utilities|Time|GetGameTimeinSeconds) (.StartTime (Utilities|Struct|BreakPrismatiscape_PulseStruct (Utilities|Array|Get(acopy) ThisPulseArray _index)))) (.Duration (Utilities|Struct|BreakPrismatiscape_PulseStruct (Utilities|Array|Get(acopy) ThisPulseArray _index)))) 1.0)
          _
          (else
            (Utilities|Array|Add (LocalVariables|GetIntsToDelete) _index)))
        (Utilities|FlowControl|Sequence
          (:then_0
            (Utilities|Array|Add StartLocAndRad (.CapsuleStartLocationAndRadius (Utilities|Struct|BreakPrismatiscape_Draw_Shape (.DrawShape (Utilities|Struct|BreakPrismatiscape_PulseStruct (Utilities|Array|Get(acopy) ThisPulseArray _index)))))))
          (:then_1
            (Utilities|Array|Add EndLocAndRad (.CapsuleEndLocationAndRadius (Utilities|Struct|BreakPrismatiscape_Draw_Shape (.DrawShape (Utilities|Struct|BreakPrismatiscape_PulseStruct (Utilities|Array|Get(acopy) ThisPulseArray _index)))))))
          (:then_2
            (Utilities|Array|Add StartVelAndStr (* (.CapsuleStartVelocityAndStrength (Utilities|Struct|BreakPrismatiscape_Draw_Shape (.DrawShape (Utilities|Struct|BreakPrismatiscape_PulseStruct (Utilities|Array|Get(acopy) ThisPulseArray _index))))) (Math|Vector4|MakeVector4 1.0 1.0 1.0 (Math|Float|Max(Float) (Math|Curves|GetFloatValue (.StrengthCurve (Utilities|Struct|BreakPrismatiscape_PulseStruct (Utilities|Array|Get(acopy) ThisPulseArray _index))) (/ (- (Utilities|Time|GetGameTimeinSeconds) (.StartTime (Utilities|Struct|BreakPrismatiscape_PulseStruct (Utilities|Array|Get(acopy) ThisPulseArray _index)))) (.Duration (Utilities|Struct|BreakPrismatiscape_PulseStruct (Utilities|Array|Get(acopy) ThisPulseArray _index))))) 0.0)))))
          (:then_3
            (Utilities|Array|Add EndVelAndStr (* (.CapsuleEndVelocityAndStrength (Utilities|Struct|BreakPrismatiscape_Draw_Shape (.DrawShape (Utilities|Struct|BreakPrismatiscape_PulseStruct (Utilities|Array|Get(acopy) ThisPulseArray _index))))) (Math|Vector4|MakeVector4 1.0 1.0 1.0 (Math|Float|Max(Float) (Math|Curves|GetFloatValue (.StrengthCurve (Utilities|Struct|BreakPrismatiscape_PulseStruct (Utilities|Array|Get(acopy) ThisPulseArray _index))) (/ (- (Utilities|Time|GetGameTimeinSeconds) (.StartTime (Utilities|Struct|BreakPrismatiscape_PulseStruct (Utilities|Array|Get(acopy) ThisPulseArray _index)))) (.Duration (Utilities|Struct|BreakPrismatiscape_PulseStruct (Utilities|Array|Get(acopy) ThisPulseArray _index))))) 0.0)))))))))
  (bind _arrayelement (Utilities|Array|ReverseforEachLoop (LocalVariables|GetIntsToDelete))
    (:LoopBody
      (Utilities|Array|RemoveIndex ThisPulseArray _arrayelement))))

(fn AddDeformPulseatLocation
  (params (PulseData :type Prismatiscape%20Pulse%20Struct%20Structure))
  (bind _we_good_ (CallFunction|IsinDrawDistance? (Math|Conversions|ToVector(Vector4) (.CapsuleStartLocationAndRadius (Utilities|Struct|BreakPrismatiscape_Draw_Shape (.DrawShape (Utilities|Struct|BreakPrismatiscape_PulseStruct PulseData)))))))
  (if _we_good_
    (Utilities|Array|Add (Variables|DataArrays|GetDeformCapsulePulses) PulseData)))

(fn DrawDeformNormals
  (Rendering|DrawMaterialtoRenderTarget 0 0))

(fn ProcessAllPulses
  (Utilities|FlowControl|Sequence
    (:then_0
      (CallFunction|ProcessPulses (Variables|DataArrays|GetDeformCapsulePulses) (Variables|Default|GetCapsuleStartLocationAndRadius) (Variables|Default|GetCapsuleEndLocationAndRadius) (Variables|Default|GetCapsuleStartVelocityAndStrength) (Variables|Default|GetCapsuleEndVelocityAndStrength)))
    (:then_1
      (CallFunction|ProcessPulses (Variables|DataArrays|GetWindCapsulePulses) (Variables|Default|GetWindCapsuleStartLocationAndRadius) (Variables|Default|GetWindCapsuleEndLocationAndRadius) (Variables|Default|GetWindCapsuleStartVelocityAndStrength) (Variables|Default|GetWindCapsuleEndVelocityAndStrength)))))

(fn SetGridTickVariables
  (Utilities|FlowControl|Sequence
    (:then_0
      (Class|NiagaraComponent|SetVariableVec2 (Variables|Default|GetNiagara) "InputGridLocation" (Math|Conversions|ToVector2D(Vector) (Transformation|GetWorldLocation (Variables|Default|GetComponentToFollow)))))
    (:then_1
      (Utilities|FlowControl|Sequence
        (:then_0
          (Class|NiagaraDataInterfaceArrayFunctionLibrary|SetNiagaraArrayVector4 (Variables|Default|GetNiagara) "CapsuleStartLocationAndRadius" (Variables|Default|GetCapsuleStartLocationAndRadius))
          (Class|NiagaraDataInterfaceArrayFunctionLibrary|SetNiagaraArrayVector4 (Variables|Default|GetNiagara) "CapsuleEndLocationAndRadius" (Variables|Default|GetCapsuleEndLocationAndRadius))
          (Class|NiagaraDataInterfaceArrayFunctionLibrary|SetNiagaraArrayVector4 (Variables|Default|GetNiagara) "CapsuleStartVelocityAndStrength" (Variables|Default|GetCapsuleStartVelocityAndStrength))
          (Class|NiagaraDataInterfaceArrayFunctionLibrary|SetNiagaraArrayVector4 (Variables|Default|GetNiagara) "CapsuleEndVelocityAndStrength" (Variables|Default|GetCapsuleEndVelocityAndStrength)))
        (:then_1
          (Class|NiagaraDataInterfaceArrayFunctionLibrary|SetNiagaraArrayVector4 (Variables|Default|GetNiagara) "WindCapsuleStartLocationAndRadius" (Variables|Default|GetWindCapsuleStartLocationAndRadius))
          (Class|NiagaraDataInterfaceArrayFunctionLibrary|SetNiagaraArrayVector4 (Variables|Default|GetNiagara) "WindCapsuleEndLocationAndRadius" (Variables|Default|GetWindCapsuleEndLocationAndRadius))
          (Class|NiagaraDataInterfaceArrayFunctionLibrary|SetNiagaraArrayVector4 (Variables|Default|GetNiagara) "WindCapsuleStartVelocityAndStrength" (Variables|Default|GetWindCapsuleStartVelocityAndStrength))
          (Class|NiagaraDataInterfaceArrayFunctionLibrary|SetNiagaraArrayVector4 (Variables|Default|GetNiagara) "WindCapsuleEndVelocityAndStrength" (Variables|Default|GetWindCapsuleEndVelocityAndStrength)))
        (:then_2
          (Class|NiagaraDataInterfaceArrayFunctionLibrary|SetNiagaraArrayVector4 (Variables|Default|GetNiagara) "InteractionBubbleLocationAndRadius" (Variables|Default|GetInteractionBubbleLocationAndRadius))
          (Class|NiagaraDataInterfaceArrayFunctionLibrary|SetNiagaraArrayVector4 (Variables|Default|GetNiagara) "InteractionBubbleVelocityAndStrength" (Variables|Default|GetInteractionBubbleVelocityAndStrength)))))))

(fn SetInitialParams
  (bind _surfaceresolution (Variables|SurfaceSimulation|GetSurfaceResolution))
  (bind _deform_resolution (Variables|DeformSettings|GetDeform%20Resolution))
  (bind _windresolution (Variables|WindSettings|GetWindResolution))
  (bind _waterresolution (Variables|WaterSettings|GetWaterResolution))
  (bind _deform_resolution_2 (Variables|DeformSettings|GetDeform%20Resolution))
  (bind _simulationinputresolution (Variables|SimulationSettings|GetSimulationInputResolution))
  (bind _waterresolution_2 (Variables|WaterSettings|GetWaterResolution))
  (bind _surfaceresolution_2 (Variables|SurfaceSimulation|GetSurfaceResolution))
  (bind _returnvalue (Math|Float|Truncate _surfaceresolution_2))
  (bind _returnvalue_2 (Math|Float|Truncate _deform_resolution))
  (bind _returnvalue_3 (Math|Float|Truncate _windresolution))
  (bind _returnvalue_4 (Math|Float|Truncate _surfaceresolution))
  (bind _returnvalue_5 (Math|Float|Truncate _simulationinputresolution))
  (bind _returnvalue_6 (Math|Float|Truncate _waterresolution))
  (bind _returnvalue_7 (Math|Float|Truncate _deform_resolution_2))
  (bind _returnvalue_8 (Math|Float|Truncate _waterresolution_2))
  (Niagara|SetNiagaraVariable(Float) (Variables|Default|GetNiagara) "TargetFPS" (Variables|Default|GetTargetFPS))
  (Class|NiagaraComponent|SetVariableInt (Variables|Default|GetNiagara) "InputGridResolution" (Math|Float|Round (Variables|SimulationSettings|GetSimulationInputResolution)))
  (Rendering|Material|SetScalarParameterValue "/Prismatiscape/Prismatiscape_MPC.Prismatiscape_MPC" "SimulationSizeWS" (Variables|SimulationSettings|GetSimulation%20SizeWS) :!class /Script/Engine.KismetMaterialLibrary)
  (Niagara|SetNiagaraVariable(Float) (Variables|Default|GetNiagara) "SimulationSizeWS" (Variables|SimulationSettings|GetSimulation%20SizeWS))
  (Utilities|FlowControl|Sequence
    (:then_0
      (Utilities|FlowControl|Sequence
        (:then_0
          (Rendering|ResizeRenderTarget2D "/Prismatiscape/RenderTargets/Prismatiscape_Deform_RT.Prismatiscape_Deform_RT" _returnvalue_7 _returnvalue_7)
          (Rendering|ResizeRenderTarget2D "/Prismatiscape/RenderTargets/Prismatiscape_InteractionBubble_RT.Prismatiscape_InteractionBubble_RT" _returnvalue_2 _returnvalue_2)
          (Rendering|ResizeRenderTarget2D "/Prismatiscape/RenderTargets/Prismatiscape_Surface_RT.Prismatiscape_Surface_RT" _returnvalue _returnvalue)
          (Rendering|ResizeRenderTarget2D "/Prismatiscape/RenderTargets/Prismatiscape_Paint_RT.Prismatiscape_Paint_RT" _returnvalue_4 _returnvalue_4))
        (:then_1
          (Rendering|ResizeRenderTarget2D "/Prismatiscape/RenderTargets/Prismatiscape_Wind_RT.Prismatiscape_Wind_RT" _returnvalue_3 _returnvalue_3))
        (:then_2
          (Rendering|ResizeRenderTarget2D "/Prismatiscape/RenderTargets/Prismatiscape_Water_RT.Prismatiscape_Water_RT" _returnvalue_8 _returnvalue_8)
          (Rendering|ResizeRenderTarget2D "/Prismatiscape/RenderTargets/Prismatiscape_WaterVelocity_RT.Prismatiscape_WaterVelocity_RT" _returnvalue_6 _returnvalue_6))
        (:then_3
          (Rendering|ResizeRenderTarget2D "/Prismatiscape/RenderTargets/Prismatiscape_DeformInput_RT.Prismatiscape_DeformInput_RT" _returnvalue_5 _returnvalue_5))))
    (:then_1
      (Utilities|FlowControl|Sequence
        (:then_0
          (Class|NiagaraComponent|SetVariableInt (Variables|Default|GetNiagara) "DeformGridResolution" (Math|Float|Round (Variables|DeformSettings|GetDeform%20Resolution)))
          (Rendering|Material|SetScalarParameterValue "/Prismatiscape/Prismatiscape_MPC.Prismatiscape_MPC" "Deform Resolution" (Variables|DeformSettings|GetDeform%20Resolution) :!class /Script/Engine.KismetMaterialLibrary))
        (:then_1
          (Class|NiagaraComponent|SetVariableInt (Variables|Default|GetNiagara) "SurfaceGridResolution" (Math|Float|Round (Variables|SurfaceSimulation|GetSurfaceResolution)))
          (Rendering|Material|SetScalarParameterValue "/Prismatiscape/Prismatiscape_MPC.Prismatiscape_MPC" "SurfaceResolution" (Variables|SurfaceSimulation|GetSurfaceResolution) :!class /Script/Engine.KismetMaterialLibrary))
        (:then_2
          (Class|NiagaraComponent|SetVariableInt (Variables|Default|GetNiagara) "WindGridResolution" (Math|Float|Round (Variables|WindSettings|GetWindResolution)))
          (Rendering|Material|SetScalarParameterValue "/Prismatiscape/Prismatiscape_MPC.Prismatiscape_MPC" "Wind Resolution" (Variables|WindSettings|GetWindResolution) :!class /Script/Engine.KismetMaterialLibrary))
        (:then_3
          (Class|NiagaraComponent|SetVariableInt (Variables|Default|GetNiagara) "WaterGridResolution" (Math|Float|Round (Variables|WaterSettings|GetWaterResolution)))
          (Rendering|Material|SetScalarParameterValue "/Prismatiscape/Prismatiscape_MPC.Prismatiscape_MPC" "Water Resolution" (Variables|WaterSettings|GetWaterResolution) :!class /Script/Engine.KismetMaterialLibrary))))))

(fn AddWindPulseatLocation
  (params (PulseData :type Prismatiscape%20Pulse%20Struct%20Structure))
  (bind _we_good_ (CallFunction|IsinDrawDistance? (Math|Conversions|ToVector(Vector4) (.CapsuleStartLocationAndRadius (Utilities|Struct|BreakPrismatiscape_Draw_Shape (.DrawShape (Utilities|Struct|BreakPrismatiscape_PulseStruct PulseData)))))))
  (if _we_good_
    (Utilities|Array|Add (Variables|DataArrays|GetWindCapsulePulses) PulseData)))

(fn CalculateRTPositionsandOffsets
  (CallFunction|CalculateDeformPosition)
  (CallFunction|CalculateSurfacePosition)
  (CallFunction|CalculateWindPosition)
  (CallFunction|CalculateWaterPosition))

(fn CalculateDeformPosition
  (bind _simulation_sizews (Variables|SimulationSettings|GetSimulation%20SizeWS))
  (bind _deform_resolution (Variables|DeformSettings|GetDeform%20Resolution))
  (bind _followlocationthisframe (Variables|Default|GetFollowLocationThisFrame))
  (bind _returnvalue (/ _simulation_sizews _deform_resolution))
  (bind (_x _y) (Math|Vector|BreakVector _followlocationthisframe))
  (Rendering|Material|SetVectorParameterValue (Variables|MPC|GetMaterialParamCollection) (Variables|Default|GetDeform%20RT%20Location%20Name) (Math|Color|MakeColor (.X (Math|Vector2D|BreakVector2D (Variables|DeformSettings|GetDeform%20Location))) (.Y (Math|Vector2D|BreakVector2D (Variables|DeformSettings|GetDeform%20Location))) 0.0 0.0) :!class /Script/Engine.KismetMaterialLibrary)
  (bind _output_get (Variables|DeformSettings|SetDeformPixelOffset (- (* (Class|KismetMathLibrary|ToRounded2D (/ (Math|Vector2D|MakeVector2D _x _y) _returnvalue)) _returnvalue) (Variables|DeformSettings|GetDeform%20Location))))
  (Variables|DeformSettings|SetDeform%20Location (+ _output_get (Variables|DeformSettings|GetDeform%20Location)))
  (Class|NiagaraComponent|SetVariableVec2 (Variables|Default|GetNiagara) "DeformGridLocation" (Variables|DeformSettings|GetDeform%20Location))
  (Class|NiagaraComponent|SetVariableVec2 (Variables|Default|GetNiagara) "DeformGridPixelOffset" (* (Variables|DeformSettings|GetDeformPixelOffset) (Math|Conversions|ToVector2D(Vector) (/ (Variables|DeformSettings|GetDeform%20Resolution) (Variables|SimulationSettings|GetSimulation%20SizeWS))) "(X=-1.000000,Y=-1.000000)")))

(fn CalculateWindPosition
  (bind _simulation_sizews (Variables|SimulationSettings|GetSimulation%20SizeWS))
  (bind _followlocationthisframe (Variables|Default|GetFollowLocationThisFrame))
  (bind _windresolution (Variables|WindSettings|GetWindResolution))
  (bind (_x _y) (Math|Vector|BreakVector _followlocationthisframe))
  (bind _returnvalue (/ _simulation_sizews _windresolution))
  (Rendering|Material|SetVectorParameterValue (Variables|MPC|GetMaterialParamCollection) (Variables|Default|GetWind%20RT%20Location%20Name) (Math|Color|MakeColor (.X (Math|Vector2D|BreakVector2D (Variables|WindSettings|GetWindLocation))) (.Y (Math|Vector2D|BreakVector2D (Variables|WindSettings|GetWindLocation))) 0.0 0.0) :!class /Script/Engine.KismetMaterialLibrary)
  (bind _output_get (Variables|WindSettings|SetWindPixelOffset (- (* (Class|KismetMathLibrary|ToRounded2D (/ (Math|Vector2D|MakeVector2D _x _y) _returnvalue)) _returnvalue) (Variables|WindSettings|GetWindLocation))))
  (Variables|WindSettings|SetWindLocation (+ _output_get (Variables|WindSettings|GetWindLocation)))
  (Class|NiagaraComponent|SetVariableVec2 (Variables|Default|GetNiagara) "WindGridLocation" (Variables|WindSettings|GetWindLocation))
  (Class|NiagaraComponent|SetVariableVec2 (Variables|Default|GetNiagara) "WindGridPixelOffset" (* (Variables|WindSettings|GetWindPixelOffset) (Math|Conversions|ToVector2D(Vector) (/ (Variables|WindSettings|GetWindResolution) (Variables|SimulationSettings|GetSimulation%20SizeWS))) "(X=-1.000000,Y=-1.000000)")))

(fn CalculateWaterPosition
  (bind _simulation_sizews (Variables|SimulationSettings|GetSimulation%20SizeWS))
  (bind _followlocationthisframe (Variables|Default|GetFollowLocationThisFrame))
  (bind _waterresolution (Variables|WaterSettings|GetWaterResolution))
  (bind (_x _y) (Math|Vector|BreakVector _followlocationthisframe))
  (bind _returnvalue (/ _simulation_sizews _waterresolution))
  (Rendering|Material|SetVectorParameterValue (Variables|MPC|GetMaterialParamCollection) (Variables|Default|GetWater%20RT%20Location%20Name) (Math|Color|MakeColor (.X (Math|Vector2D|BreakVector2D (Variables|WaterSettings|GetWaterLocation))) (.Y (Math|Vector2D|BreakVector2D (Variables|WaterSettings|GetWaterLocation))) 0.0 0.0) :!class /Script/Engine.KismetMaterialLibrary)
  (bind _output_get (Variables|WaterSettings|SetWaterPixelOffset (- (* (Class|KismetMathLibrary|ToRounded2D (/ (Math|Vector2D|MakeVector2D _x _y) _returnvalue)) _returnvalue) (Variables|WaterSettings|GetWaterLocation))))
  (Variables|WaterSettings|SetWaterLocation (+ _output_get (Variables|WaterSettings|GetWaterLocation)))
  (Class|NiagaraComponent|SetVariableVec2 (Variables|Default|GetNiagara) "WaterGridLocation" (Variables|WaterSettings|GetWaterLocation))
  (Class|NiagaraComponent|SetVariableVec2 (Variables|Default|GetNiagara) "WaterGridPixelOffset" (* (Variables|WaterSettings|GetWaterPixelOffset) (Math|Conversions|ToVector2D(Vector) (/ (Variables|WaterSettings|GetWaterResolution) (Variables|SimulationSettings|GetSimulation%20SizeWS))) "(X=-1.000000,Y=-1.000000)")))

(fn CalculateSurfacePosition
  (bind _simulation_sizews (Variables|SimulationSettings|GetSimulation%20SizeWS))
  (bind _surfaceresolution (Variables|SurfaceSimulation|GetSurfaceResolution))
  (bind _followlocationthisframe (Variables|Default|GetFollowLocationThisFrame))
  (bind _returnvalue (/ _simulation_sizews _surfaceresolution))
  (bind (_x _y) (Math|Vector|BreakVector _followlocationthisframe))
  (Rendering|Material|SetVectorParameterValue (Variables|MPC|GetMaterialParamCollection) (Variables|Default|GetSurface%20RT%20Location%20Name) (Math|Color|MakeColor (.X (Math|Vector2D|BreakVector2D (Variables|SurfaceSimulation|GetSurface%20Location))) (.Y (Math|Vector2D|BreakVector2D (Variables|SurfaceSimulation|GetSurface%20Location))) 0.0 0.0) :!class /Script/Engine.KismetMaterialLibrary)
  (bind _output_get (Variables|SurfaceSimulation|SetSurfacePixelOffset (- (* (- (Class|KismetMathLibrary|ToRounded2D (/ (Math|Vector2D|MakeVector2D _x _y) _returnvalue)) "(X=-0.500000,Y=-0.500000)") _returnvalue) (Variables|SurfaceSimulation|GetSurface%20Location))))
  (Variables|SurfaceSimulation|SetSurface%20Location (+ _output_get (Variables|SurfaceSimulation|GetSurface%20Location)))
  (Class|NiagaraComponent|SetVariableVec2 (Variables|Default|GetNiagara) "SurfaceGridLocation" (Variables|SurfaceSimulation|GetSurface%20Location))
  (Class|NiagaraComponent|SetVariableVec2 (Variables|Default|GetNiagara) "SurfaceGridPixelOffset" (* (Variables|SurfaceSimulation|GetSurfacePixelOffset) (Math|Conversions|ToVector2D(Vector) (/ (Variables|SurfaceSimulation|GetSurfaceResolution) (Variables|SimulationSettings|GetSimulation%20SizeWS))) "(X=-1.000000,Y=-1.000000)")))

(fn IsinDrawDistance?
  (params (TheFellasLocation :type Vector))
  (bind _componenttofollow (Variables|Default|GetComponentToFollow))
  (Utilities|IsValid _componenttofollow
    (:Is%20Valid
      (return (< (Class|KismetMathLibrary|VectorDistance2DSquared (Transformation|GetWorldLocation _componenttofollow) TheFellasLocation) (Math|Float|Square (* (Variables|SimulationSettings|GetSimulation%20SizeWS) 0.75)))))))

(fn UpdateVisibility
  (params (VisCycle :type Integer%20%28by%20ref%29) (TargetArray :type Array%20of%20Prismatiscape%20Draw%20Component%20Object%20References))
  (bind _output (Utilities|Array|Get(acopy) TargetArray VisCycle))
  (Utilities|FlowControl|Sequence
    (:then_0
      (if (Utilities|Array|IsValidIndex TargetArray VisCycle)
        (Utilities|IsValid _output
          (:Is%20Valid
            (bind _we_good_ (CallFunction|IsinDrawDistance? (Transformation|GetActorLocation (Components|GetOwner _output))))
            (Variables|/Script/Prismatiscape.PrismatiscapeDrawComponent|SetbIsVisible _output _we_good_)))
        (else
          (|SetBy-RefVar VisCycle -1))))
    (:then_1
      (Math|Integer|IncrementInt VisCycle))))

(fn InitComponenttoFollow
  (bind _returnvalue (Game|Player|GetPlayerPawn 0))
  (bind _rootcomponent (Variables|/Script/Engine.Actor|GetRootComponent _returnvalue))
  (Utilities|IsValid _returnvalue
    (:Is%20Valid
      (Utilities|IsValid _rootcomponent
        (:Is%20Valid
          (Variables|Default|SetComponentToFollow _rootcomponent))))))

(fn UpdateAllVisibilities
  (Utilities|FlowControl|Sequence
    (:then_0
      (if (Utilities|Array|IsValidIndex (Variables|Default|GetDeformComponents))
        (CallFunction|UpdateVisibility (Variables|Default|GetDeformVisibilityCycle) (Variables|Default|GetDeformComponents))))
    (:then_1
      (if (Utilities|Array|IsValidIndex (Variables|Default|GetWindComponents))
        (CallFunction|UpdateVisibility (Variables|Default|GetWindVisibilityCycle) (Variables|Default|GetWindComponents))))
    (:then_2
      (if (Utilities|Array|IsValidIndex (Variables|Default|GetInteractionBubbleComponents))
        (CallFunction|UpdateVisibility (Variables|Default|GetBubbleVisibilityCycle) (Variables|Default|GetInteractionBubbleComponents))))))

(fn ReplaceCurrentStyleProfile
  (params (StyleProfile :type Prismatiscape%20Style%20Profile%20Object%20Reference))
  (for (_array_element _array_index) (Variables|Default|GetCurrentSimulationStyles)
    (if (== (Utilities|GetClass _array_element) (Utilities|GetClass StyleProfile))
      (Utilities|Array|SetArrayElem (Variables|Default|GetCurrentSimulationStyles) _array_index StyleProfile)
      (return)))
  (Utilities|Array|Add (Variables|Default|GetCurrentSimulationStyles) StyleProfile))

(fn BPHashInteractionBubbles
  (params (BubblePositionAndRadius :type Array%20of%20Vector%204%20Structures) (BubbleVelocityAndStrength :type Array%20of%20Vector%204%20Structures))
  (for _array_element BubblePositionAndRadius
    (bind _gridindices (CallFunction|GridIndexesfromLocation (Math|Conversions|ToVector(Vector4) _array_element)))
    (for _array_element_2 _gridindices
      _)))

(fn BPGridIndexesfromLocation
  (params (Location :type Vector))
  (bind _returnvalue (Math|Conversions|ToVector2D(Vector) Location))
  (bind _simulation_sizews (Variables|SimulationSettings|GetSimulation%20SizeWS))
  (bind _followlocationthisframe (Variables|Default|GetFollowLocationThisFrame))
  (bind _simulation_sizews_2 (Variables|SimulationSettings|GetSimulation%20SizeWS))
  (bind _bp_hashgriddimension (Variables|Default|GetBP_HashGridDimension))
  (bind _returnvalue_2 (Math|Conversions|ToVector2D(Vector) _followlocationthisframe))
  (bind _returnvalue_3 (/ _simulation_sizews _bp_hashgriddimension))
  (bind _returnvalue_4 (/ _simulation_sizews_2 2.0))
  (bind _returnvalue_5 (- _returnvalue_2 _returnvalue_4))
  (bind _returnvalue_6 (- _returnvalue _returnvalue_5))
  (bind _returnvalue_7 (/ _returnvalue_6 _returnvalue_3))
  (bind (_x _y) (Math|Vector2D|BreakVector2D _returnvalue_7))
  (return (Utilities|Array|MakeArray (+ (* (Variables|Default|GetBP_HashGridDimension) (Math|Float|Round _x)) (Math|Float|Round _y)))))