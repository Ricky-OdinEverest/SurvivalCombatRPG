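; GA_SimpleMelee is a melee gameplay ability that faces the avatar toward its combat target and plays a random tagged attack montage.
; When the montage's tagged gameplay event arrives, it gets the matching combat socket location and finds live players within a small radius.
; It damages non-friendly hits, then ends; montage completion, interruption or cancellation also ends it.
; The montage can continue after the ability ends.
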(event Ability|EventActivateAbility
  (Variables|Default|SetAbilitySourceActor (Ability|GetAvatarActorfromActorInfo))
  (bind _returnvalue (Class|EnemyInterface|GetCombatTarget(Message) (Variables|Default|GetAbilitySourceActor)))
  (bind _ascombat_interface (Utilities|Casting|CastToCombatInterface (Variables|Default|GetAbilitySourceActor)))
  (Class|CombatInterface|UpdateFacingTarget _ascombat_interface (Transformation|GetActorLocation _returnvalue))
  (bind _returnvalue_2 (Class|CombatInterface|GetAttackMontages(Message) (Variables|Default|GetAbilitySourceActor)))
  (bind _output_get (Variables|Default|SetTagged%20Montage (Utilities|Array|Get(acopy) _returnvalue_2 (Math|Random|RandomIntegerinRange 0 (- (Utilities|Array|Length _returnvalue_2) 1)))))
  (Variables|Default|SetMontage%20Tag (.MontageTag (Utilities|Struct|BreakTaggedMontage _output_get)))
  (|PlayMontageandWaitProxy "None" (.Montage (Utilities|Struct|BreakTaggedMontage _output_get)) 1.0 "None" false 1.0 0.0 false
    (:then
      (Ability|Tasks|WaitGameplayEvent (Variables|Default|GetMontage%20Tag) 0
        (:EventReceived
          (bind _returnvalue_3 (Class|CombatInterface|GetCombatSocketLocation(Message) (Variables|Default|GetAbilitySourceActor) (Variables|Default|GetMontage%20Tag)))
          (bind _outoverlappingactors (Class|SCRAbilitySystemLibrary|GetLivePlayersWithinRadius (Variables|Default|GetAbilitySourceActor) (Utilities|Array|MakeArray (Variables|Default|GetAbilitySourceActor)) 3e+01 _returnvalue_3))
          (for _array_element _outoverlappingactors
            (if (Class|SCRAbilitySystemLibrary|IsNotFriend (Variables|Default|GetAbilitySourceActor) _array_element)
              (Class|SCRDamageGameplayAbility|CauseDamage _array_element)))
          (Ability|EndAbility))))
    (:OnCompleted
      (Ability|EndAbility :!label _label))
    (:OnInterrupted
      (goto _label))
    (:OnCancelled
      (goto _label))))