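; Gameplay ability that casts a player-aimed Fire Bolt projectile.
; A TargetFromPlayer task supplies the hit location, which turns the avatar to face it through CombatInterface before a left-hand cast montage plays.
; The montage's FireBolt gameplay event triggers SpawnProjectile toward that location, then the ability ends after a short delay.
; Montage completion, interruption or cancellation also ends it.
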(event Ability|EventActivateAbility
  (bind _datahandle (|TargetfromPlayer)
    (:ValidData
      (Variables|Default|SetProjectileTargetLocation (.Location (Collision|BreakHitResult (Ability|TargetData|GetHitResultfromTargetData _datahandle))))
      (bind _ascombat_interface (Utilities|Casting|CastToCombatInterface (Ability|GetAvatarActorfromActorInfo)))
      (Class|CombatInterface|UpdateFacingTarget _ascombat_interface (Variables|Default|GetProjectileTargetLocation))
      (|PlayMontageandWaitProxy "None" "/Game/Assets/SAM_AnimLibrary/S_AM_HumanLeftHandSpellCast_SAM.S_AM_HumanLeftHandSpellCast_SAM" 1.0 "" true 1.0 0.0 true
        (:then
          (Ability|Tasks|WaitGameplayEvent "(TagName=\"Event.Montage.FireBolt\")" 0
            (:EventReceived
              (Class|SCRProjectileSpell|SpawnProjectile (Variables|Default|GetProjectileTargetLocation) (Variables|Default|GetMontage%20Tag))
              (Utilities|FlowControl|Delay 0.2)
              (Ability|EndAbility))))
        (:OnCompleted
          (Ability|EndAbility :!label _label))
        (:OnInterrupted
          (goto _label))
        (:OnCancelled
          (goto _label))))))

(event Ability|EventOnEndAbility
  (params (bWasCancelled :type Boolean)))