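; Vault component for the player character that detects climbable ledges, shows a prompt widget, and moves the player onto them.
; While idle, Tick traces vertically ahead of the capsule and validates hit height, surface walkability and capsule clearance to store a landing point.
; Vault records the start location and switches state, then Tick lerps the owner to that point with non-swept teleports.
; Debug drawing and height printing remain enabled.
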(event Custom|Vault
  (Variables|Default|SetProgress 0.0)
  (Variables|Default|SetStartingLocation (Transformation|GetActorLocation (Variables|Default|GetOwningCharacter)))
  (Variables|Default|SetVaultingState "NewEnumerator2"))

(event EventBeginPlay
  (bind _asbp_player_character (Utilities|Casting|CastToBP_PlayerCharacter (Components|GetOwner)))
  (Variables|Default|SetOwningCharacter _asbp_player_character)
  (bind _returnvalue (UserInterface|CreateWidget "/Game/Blueprints/UI/WBP_VaultPrompt.WBP_VaultPrompt_C" (.AsBP%20Player%20Controller (Utilities|Casting|CastToBP_PlayerController (Pawn|GetController (Variables|Default|GetOwningCharacter))))))
  (Variables|Default|SetVaultWidget _returnvalue))

(event EventTick
  (params (DeltaSeconds :type Float%20%28single-precision%29))
  (bind _vaultwidget (Variables|Default|GetVaultWidget))
  (bind _vaultwidget_2 (Variables|Default|GetVaultWidget))
  (Utilities|SwitchVaultingState
    (:NotVaulting
      (bind (_result _endinglocaiton) (CallFunction|CanVault))
      (if _result
        (Variables|Default|SetEnding%20Locaiton _endinglocaiton)
        (if (not (UserInterface|Viewport|IsinViewport _vaultwidget_2))
          (UserInterface|Viewport|AddtoViewport _vaultwidget_2 0))
        (elif (UserInterface|Viewport|IsinViewport _vaultwidget)
          (Widget|RemovefromParent _vaultwidget))))
    (:Vaulting
      (CallFunction|TickVault DeltaSeconds))))

(fn CanVault
  (bind _owningcharacter (Variables|Default|GetOwningCharacter))
  (bind _returnvalue (Transformation|GetActorLocation _owningcharacter))
  (bind _returnvalue_2 (Transformation|GetActorForwardVector _owningcharacter))
  (bind _returnvalue_3 (* _returnvalue_2 7e+01))
  (bind _returnvalue_4 (+ _returnvalue _returnvalue_3))
  (if (Utilities|Enum|Equal(Enum) (Variables|Default|GetVaultingState) "NewEnumerator0")
    (LocalVariables|SetCaspsule%20%28local%29 (Variables|/Script/Engine.Character|GetCapsuleComponent (Variables|Default|GetOwningCharacter)))
    (bind (_outhit _returnvalue_5) (Collision|LineTraceByChannel (+ _returnvalue_4 (Math|Vector|MakeVector 0.0 0.0 (Components|Capsule|GetScaledCapsuleHalfHeight (LocalVariables|GetCaspsule%20%28local%29)))) (- _returnvalue_4 (Math|Vector|MakeVector 0.0 0.0 (Components|Capsule|GetScaledCapsuleHalfHeight (LocalVariables|GetCaspsule%20%28local%29)))) "TraceTypeQuery1" false (Utilities|Array|MakeArray (Variables|Default|GetOwningCharacter)) "ForOneFrame"))
    (if _returnvalue_5
      (bind (_bcanvaulttohit _ending_location) (CallFunction|CanVaulttoHit (LocalVariables|GetCaspsule%20%28local%29) _outhit))
      (return _bcanvaulttohit _ending_location)
      (else
        (return false "0, 0, 0")))
    (else
      (return false "0, 0, 0"))))

(fn CanVaulttoHit
  (params (Capsule :type Capsule%20Component%20Object%20Reference) (hit :type Hit%20Result%20Structure))
  (bind _returnvalue (Components|Capsule|GetScaledCapsuleHalfHeight Capsule))
  (bind _returnvalue_2 (Components|Capsule|GetScaledCapsuleRadius Capsule))
  (bind _z (Math|Vector|BreakVector (.location hit)))
  (bind _z_2 (Math|Vector|BreakVector (.traceend hit)))
  (bind _returnvalue_3 (- _z _z_2))
  (Utilities|FlowControl|Sequence
    (:then_0
      (Development|PrintString (Utilities|String|ToString(Float) _returnvalue_3) true true "(R=0.000000,G=0.660000,B=1.000000,A=1.000000)" 0.0 "1")
      (if (not (Math|Float|InRange(Float) _returnvalue_3 (Variables|Default|GetMinVaultingHeight) (Variables|Default|GetMaxVaultingHeight)))
        (return false "0, 0, 0")))
    (:then_1
      (if (< (.Z (Math|Vector|BreakVector (.normal hit))) (Class|CharacterMovementComponent|GetWalkableFloorZ (Variables|/Script/Engine.Character|GetCharacterMovement (Variables|Default|GetOwningCharacter))))
        (return false "0, 0, 0")))
    (:then_2
      (bind _output_get (LocalVariables|SetEndingLocation%28Local%29 (+ (.location hit) (Math|Vector|MakeVector 0.0 0.0 _returnvalue))))
      (bind _result (CallFunction|CheckCapsuleCollision (+ _output_get (Math|Vector|MakeVector 0.0 0.0 _returnvalue_2)) _returnvalue _returnvalue_2 true))
      (if _result
        (return false "0, 0, 0")))
    (:then_3
      (return true (LocalVariables|GetEndingLocation%28Local%29)))))

(fn CheckCapsuleCollision
  (params (Center :type Vector) (HalfHeight :type Float%20%28double-precision%29) (Radius :type Float%20%28double-precision%29) (DrawDebug :type Boolean))
  (Utilities|FlowControl|Sequence
    (:then_0
      (if DrawDebug
        (Rendering|Debug|DrawDebugCapsule Center HalfHeight Radius "0, 0, 0" "(R=1.000000,G=0.933011,B=0.000000,A=1.000000)" 0.0 3.0)))
    (:then_1
      (bind _returnvalue (Collision|CapsuleOverlapActors Center Radius HalfHeight (Utilities|Array|MakeArray "ObjectTypeQuery1" "ObjectTypeQuery2" "ObjectTypeQuery4" "ObjectTypeQuery5" "ObjectTypeQuery6") "/Script/Engine.Actor" (Utilities|Array|MakeArray (Variables|Default|GetOwningCharacter))))
      (return _returnvalue))))

(fn TickVault
  (params (DeltaSeconds :type Float%20%28double-precision%29))
  (Utilities|FlowControl|Sequence
    (:then_0
      (Variables|Default|SetProgress (Math|Float|Clamp(Float) (+ (Variables|Default|GetProgress) (/ DeltaSeconds (Variables|Default|GetVaultSpeed)))))
      (Transformation|SetActorLocation (Variables|Default|GetOwningCharacter) (Math|Vector|Lerp(Vector) (Variables|Default|GetStartingLocation) (Variables|Default|GetEnding%20Locaiton) (Variables|Default|GetProgress)) false true))
    (:then_1
      (if (>= (Variables|Default|GetProgress) 1.0)
        (Variables|Default|SetVaultingState "NewEnumerator0")))))