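; Player character Blueprint with a NinjaSuit following the main mesh's pose, a motion-warp facing target, and helpers for runtime vertex painting.
; A camera aim trace uses a server-cached yaw to orient the boom for remote proxies, since base aim yaw isn't replicated.
; The paint helper capsule-traces unique meshes around a hit, then paints each with combined color detection and a drying-pause flag.
; The graph chaining trace into paint is disconnected.
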(event EventBeginPlay)

(event Collision|EventActorBeginOverlap
  (params (OtherActor :type Actor%20Object%20Reference)))

(event EventTick
  (params (DeltaSeconds :type Float%20%28single-precision%29)))

(event EventUpdateFacingTarget
  (params (Target :type Vector%20%28by%20ref%29 :default "0, 0, 0"))
  (Class|MotionWarpingComponent|AddorUpdateWarpTargetfromLocation (Variables|Default|GetMotionWarping) "FacingTarget" Target))

(event Input|MouseEvents|LeftMouseButton
  (params (Key :type Key%20Structure :default "None")))

(event Input|GamepadEvents|GamepadFaceButtonLeft
  (params (Key :type Key%20Structure :default "None")))

(fn ConstructionScript
  (Components|SkinnedMesh|SetLeaderPoseComponent (Variables|Default|GetNinjaSuit) (Variables|Character|GetMesh) true false))

(fn GetHitResultUnderCursor
  (bind _asplayer_controller (Utilities|Casting|CastToPlayerController (Pawn|GetController self)))
  (return (.bBlockingHit (Collision|BreakHitResult (.HitResult (Game|Player|GetHitResultUnderCursorbyChannel _asplayer_controller "TraceTypeQuery1" true)))) (.Location (Collision|BreakHitResult (.HitResult (Game|Player|GetHitResultUnderCursorbyChannel _asplayer_controller "TraceTypeQuery1" true))))))

(fn SingleTraceForwardfromCamera
  (bind _returnvalue (Pawn|GetBaseAimRotation))
  (bind _followcamera (Variables|Default|GetFollowCamera))
  (bind _returnvalue_2 (Transformation|GetWorldLocation _followcamera))
  (Utilities|FlowControl|Sequence
    (:then_0
      (Networking|SwitchHasAuthority
        (:Authority
          (Variables|Default|SetplayerBaseAimRotationYaw (.yaw (Pawn|GetBaseAimRotation))) ; The yaw isn't replicated from base aim rotation
        )))
    (:then_1
      (if (or (Ability|HasAuthority) (Pawn|IsLocallyControlled))
        (Variables|Default|SetaimRotationTemp (Pawn|GetBaseAimRotation))
        (bind (_outhit _returnvalue_3) (Collision|LineTraceByChannel _returnvalue_2 (+ _returnvalue_2 (* (Math|Vector|GetForwardVector (Variables|Default|GetaimRotationTemp)) 1e+05)) "TraceTypeQuery1" true 0 "ForDuration" true "(R=1.000000,G=0.000000,B=0.000000,A=1.000000)" "(R=0.000000,G=1.000000,B=0.000000,A=1.000000)" 0.2))
        (return _returnvalue_3 _outhit)
        (else
          (Transformation|SetWorldRotation (Variables|Default|GetCameraBoom) (Math|Rotator|MakeRotator (.roll _returnvalue) (.pitch _returnvalue) (Variables|Default|GetplayerBaseAimRotationYaw)) false false)
          (Variables|Default|SetaimRotationTemp (Math|Rotator|MakeRotator (.roll _returnvalue) (.pitch _returnvalue) (Variables|Default|GetplayerBaseAimRotationYaw))))))))

(fn PaintatLocationwithHitResult
  (params (Hit :type Hit%20Result%20Structure%20%28by%20ref%29) (Paint%20at%20Location%20Struct%20Area%20Of%20EffectRangeStart :type Float%20%28single-precision%29) (Paint%20at%20Location%20Struct%20Area%20Of%20EffectRangeEnd :type Float%20%28single-precision%29) (Paint%20at%20Location%20Struct%20Fall%20Off%20Strength :type Float%20%28single-precision%29) (Paint%20at%20Location%20Struct%20Strength%20To%20Apply%20On%20Colors :type RVPDP%20Apply%20Color%20Settings%20Structure) (Distance%20to%20Base%20Falloff%20From :type Float%20%28single-precision%29) (Fall%20Off%20Type :type EVertexPaintAtLocationFallOffType%20Enum :default "OutwardFallOff"))
  (bind (_bblockinghit _binitialoverlap _time _distance _location _impactpoint _normal _impactnormal _physmat _hitactor _hitcomponent _hitbonename) (Collision|BreakHitResult Hit))
  ;[1 1 1] Paint at Location with Hit Result
  (bind (_closestuniquemesheswithbones _returnvalue) (|MultiCapsuleTraceforUniqueMeshes (.Location (Collision|BreakHitResult Hit)) 0.0 "TraceTypeQuery1" "ObjectTypeQuery1" (Utilities|Array|MakeArray self) false false "None" 0.2))
  (if _returnvalue
    (for _array_element _closestuniquemesheswithbones
      (|PaintatLocationNode (Variables|Default|GetVertexPaintDetection) (.HitComponent (Collision|BreakHitResult (.ClosestHitResultOfMesh (Utilities|Struct|BreakRVPDPTraceForClosestUniqueMeshesAndBonesPrerequisite _array_element)))) (Utilities|Struct|MakeRVPDPPaintAtLocationSettings (Utilities|Struct|MakeRVPDPAtLocationTasksSettings (.Location (Collision|BreakHitResult (.ClosestHitResultOfMesh (Utilities|Struct|BreakRVPDPTraceForClosestUniqueMeshesAndBonesPrerequisite _array_element)))) (.Normal (Collision|BreakHitResult (.ClosestHitResultOfMesh (Utilities|Struct|BreakRVPDPTraceForClosestUniqueMeshesAndBonesPrerequisite _array_element)))) (.HitBoneName (Collision|BreakHitResult (.ClosestHitResultOfMesh (Utilities|Struct|BreakRVPDPTraceForClosestUniqueMeshesAndBonesPrerequisite _array_element))))) (Utilities|Struct|MakeRVPDPPaintAtLocationAreaOfEffectSettings Paint%20at%20Location%20Struct%20Area%20Of%20EffectRangeStart Paint%20at%20Location%20Struct%20Area%20Of%20EffectRangeEnd (Utilities|Struct|MakeRVPDPPaintAtLocationFallOffSettings Fall%20Off%20Type Paint%20at%20Location%20Struct%20Fall%20Off%20Strength "BaseOfPaintShape" Distance%20to%20Base%20Falloff%20From) (Utilities|Struct|MakeRVPDPGetAverageColorSettings true Paint%20at%20Location%20Struct%20Area%20Of%20EffectRangeEnd -1.0) (.MeshBonesWithinTrace (Utilities|Struct|BreakRVPDPTraceForClosestUniqueMeshesAndBonesPrerequisite _array_element))) (Utilities|Struct|MakeRVPDPEstimatedColorAtHitLocationSettings false true 60000 0.25) (Utilities|Struct|MakeRVPDPGetClosestVertexDataComboPaintAtLocationSettings false (Utilities|Struct|MakeRVPDPGetAverageColorSettings true 1.5e+02 -1.0) true (Utilities|Struct|MakeRVPDPAtLocationTasksSettings _location _normal _hitbonename)) Paint%20at%20Location%20Struct%20Strength%20To%20Apply%20On%20Colors true "(OverrideLODToPaintUpTo=False,AmountOfLODsToPaint=1)" true 0 "(OverrideVertexColorsToApply=False,ObjectToRunOverrideVertexColorsInterface=None,OverrideVertexColorsToApplyID=0,OnlyRunOverrideInterfaceIfTryingToApplyColorToVertex=True,IncludeMostDominantPhysicsSurface=False)" "(IncludeBonesThatGotPainted=False,IncludePaintedVertexIndicesAtLOD0=False)" (.HitItem (Collision|BreakHitResult (.ClosestHitResultOfMesh (Utilities|Struct|BreakRVPDPTraceForClosestUniqueMeshesAndBonesPrerequisite _array_element))))) (Utilities|Struct|MakeRVPDPAdditionalDataToPassThroughInfo 0 0 0 0 false (Class|KismetSystemLibrary|MakeLiteralBool true))))))