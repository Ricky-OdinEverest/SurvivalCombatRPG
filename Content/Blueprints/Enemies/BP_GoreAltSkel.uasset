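; BP_GoreAltSkel is an enemy Blueprint that hooks its skeletal mesh into a gore system.
; On BeginPlay it runs the parent logic, then initializes the UEGoreSystem component with Mesh.
; An unconnected debug chain would set the gore system's visual mesh from the first cosmetic character part.
; The OnCharacterPartsChanged event is empty, so that chain never runs.
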(event OnCharacterPartsChanged(B_PawnCosemeticThingy)
  (params (ComponentWithChangedParts :type SCR%20Pawn%20Component%20Character%20Parts%20Object%20Reference)))

(event EventBeginPlay
  (|CallParentFunction)
  (Class|UEGoreSystemComponent|Init (Variables|Default|GetUEGoreSystem) (Variables|Character|GetMesh)))

(event Collision|EventActorBeginOverlap
  (params (OtherActor :type Actor%20Object%20Reference))
  (|CallParentFunction OtherActor) ; This node is disabled and will not be called.\nDrag off pins to build functionality.
)

(event EventTick
  (params (DeltaSeconds :type Float%20%28single-precision%29))
  (|CallParentFunction DeltaSeconds) ; This node is disabled and will not be called.\nDrag off pins to build functionality.
)

(fn ConstructionScript
  (|CallParentFunction))